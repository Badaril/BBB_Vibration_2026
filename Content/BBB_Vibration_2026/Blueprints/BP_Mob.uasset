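; BP_Mob is a melee enemy that walks to locations received through ReceiveHeartBeat and attacks the player at close range.
; Tick checks player distance to trigger an attack montage with a growl, toggling Sphere active during a timed window.
; Sphere overlaps damage BP_MainCharacter.
; At zero Hp it ragdolls, destroys Sphere, disables capsule collision, plays another growl and calls JeMort on the player.
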(event `self.ReceiveBeginPlay`
  (`ActorComponent.SetActive` (`self.Sphere`) false false))

(event `self.ReceiveTick`
  (params (DeltaSeconds :type "Float (single-precision)"))
  (if (not (`self.isDead`))
    (`|ExecutionSequence`
      (:`then_0`
        (if (and (not (`self.IsAttacking?`)) (<= (`KismetMathLibrary.VSize` (- (`self.K2_GetActorLocation` (`GameplayStatics.GetPlayerCharacter` 0)) (`self.K2_GetActorLocation`))) 150.0))
          (set `self.IsAttacking?` true)
          (`self.Attack`)))
      (:`then_1`
        (`KismetSystemLibrary.Delay` 4.0)))))

(event `Attack`
  (bind _sphere (`self.Sphere`))
  (`|ExecutionSequence`
    (:`then_0`
      (`|PlayMontage` (`self.Mesh`) "/Game/BBB_Vibration_2026/Assets/MOB/anims/Mob_BBB_Anim_Armature_Attack_Montage.Mob_BBB_Anim_Armature_Attack_Montage"
        (:`then`
          (`KismetSystemLibrary.Delay` 0.3)
          (`ActorComponent.SetActive` _sphere true false)
          (`KismetSystemLibrary.Delay` 0.6)
          (`ActorComponent.SetActive` _sphere false false))
        (:`OnCompleted`
          (set `self.IsAttacking?` false))))
    (:`then_1`
      (`KismetSystemLibrary.Delay` 0.2)
      (`AudioComponent.Play` (`self.monster-growl-390285`) 0.0))))

(event `Receive HeartBeat`
  (params (Location :type "Vector Structure"))
  (if (`self.isDead`)
    _
    (elif (not (`self.IsAttacking?`))
      (`|AIMoveTo` self Location null 100.0))))

(event `self.Sphere.OnComponentBeginOverlap`
  (params (OverlappedComponent :type "PrimitiveComponent Object Reference") (OtherActor :type "Actor Object Reference") (OtherComp :type "PrimitiveComponent Object Reference") (OtherBodyIndex :type Integer) (bFromSweep :type Boolean) (SweepResult :type "HitResult Structure (by ref)"))
  (if (not (`self.isDead`))
    (bind _asbp_main_character (cast `/Game/BBB_Vibration_2026/Blueprints/BP_MainCharacter` OtherActor))
    (`/Game/BBB_Vibration_2026/Blueprints/BP_MainCharacter.TakeDamage` _asbp_main_character 1)))

(event `Take damage`
  (params (Value :type Integer))
  (bind _returnvalue (- (`self.Hp`) Value))
  (bind _output_get (set `self.Hp` _returnvalue))
  (`KismetSystemLibrary.PrintString` (`KismetStringLibrary.Conv_IntToString` _returnvalue) true true (struct :`R` 1.0 :`G` 0.220338 :`A` 1.0))
  (if (<= _output_get 0)
    (`self.Dies`)))

(event `Dies`
  (bind _monster_growl_390285 (`self.monster-growl-390285`))
  (`PrimitiveComponent.SetSimulatePhysics` (`self.Mesh`) true)
  (`ActorComponent.K2_DestroyComponent` (`self.Sphere`))
  (bind _asbp_main_character (cast `/Game/BBB_Vibration_2026/Blueprints/BP_MainCharacter` (`GameplayStatics.GetPlayerCharacter` 0)))
  (`/Game/BBB_Vibration_2026/Blueprints/BP_MainCharacter.JeMort` _asbp_main_character)
  (`AudioComponent.SetSound` _monster_growl_390285 "/Game/BBB_Vibration_2026/Sound/monster-growl-382706.monster-growl-382706")
  (`AudioComponent.SetPitchMultiplier` _monster_growl_390285 1.0)
  (`AudioComponent.Play` _monster_growl_390285 0.0)
  (`PrimitiveComponent.SetCollisionEnabled` (`self.CapsuleComponent`) "NoCollision")
  (set `self.isDead` true))

(fn `UserConstructionScript`)