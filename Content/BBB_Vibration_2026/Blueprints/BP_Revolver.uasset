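; BP_Revolver is a revolver that fires and reloads by binding to the shooting and reloading events of the player character's weapon component.
; Each shot line-traces from the cylinder along the arrow with debug drawing, spawns a bullet, decrements ammo and destroys that bullet if the trace hit a BP_Mob.
; Reloading adds one round up to the maximum.
; Ammo and mob hits only print to screen; no damage is applied here.
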(event `Reloading`
  (bind _output_get (set `self.Ammo` (`KismetMathLibrary.Clamp` (+ (`self.Ammo`) 1) 0 (`self.MaxAmmo`))))
  (`KismetSystemLibrary.PrintString` (`KismetStringLibrary.Conv_IntToString` _output_get)))

(event `self.ReceiveBeginPlay`
  (bind _asbp_main_character (cast `/Game/BBB_Vibration_2026/Blueprints/BP_MainCharacter` (`GameplayStatics.GetPlayerPawn` 0)))
  (bind _bpc_weapon (`/Game/BBB_Vibration_2026/Blueprints/BP_MainCharacter.BPC_Weapon` _asbp_main_character))
  (add `/Game/BBB_Vibration_2026/Blueprints/BPC_Weapon.Shooting` _bpc_weapon (delegate `Shooting`))
  (add `/Game/BBB_Vibration_2026/Blueprints/BPC_Weapon.Reloading` _bpc_weapon (delegate `Reloading`)))

(event `Shooting`
  (bind _returnvalue (`SceneComponent.K2_GetComponentLocation` (`self.Cylinder`)))
  (if (> (`self.Ammo`) 0)
    (bind _outhit (`KismetSystemLibrary.LineTraceSingle` :`Start` _returnvalue :`End` (+ (* (`SceneComponent.GetForwardVector` (`self.Arrow`)) 10000.0) _returnvalue) :`TraceChannel` "TraceTypeQuery1" :`DrawDebugType` "ForDuration"))
    (bind _returnvalue_2 (`|SpawnActorFromClass` "/Game/BBB_Vibration_2026/Blueprints/BP_Bullet.BP_Bullet_C" (`SceneComponent.K2_GetComponentToWorld` (`self.SpawnProjectileLocation`)) "Undefined" "MultiplyWithRoot" null null))
    (bind _output_get (set `self.Ammo` (`KismetMathLibrary.Clamp` (+ (`self.Ammo`) -1) 0 (`self.MaxAmmo`))))
    (`KismetSystemLibrary.PrintString` (`KismetStringLibrary.Conv_IntToString` _output_get))
    (cast `/Game/BBB_Vibration_2026/Blueprints/BP_Mob` (`.HitActor` (`GameplayStatics.BreakHitResult` _outhit)))
    (`KismetSystemLibrary.PrintString` "Ok")
    (`self.K2_DestroyActor` _returnvalue_2)))

(fn `UserConstructionScript`)