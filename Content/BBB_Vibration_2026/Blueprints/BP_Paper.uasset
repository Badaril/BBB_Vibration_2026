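; Paper note actor whose Index selects both the plane's material at construction and the content value passed to its text screen.
; Entering the sphere caches BP_MainCharacter and shows the Widget component; leaving hides it and calls TakeCollectible on the character as non-ammo, with Value and Adrenaline.
; OpenText and CloseText, not called within this Blueprint, add and remove the WBP_Text viewport widget.
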(event `self.Sphere.OnComponentBeginOverlap`
  (params (OverlappedComponent :type "PrimitiveComponent Object Reference") (OtherActor :type "Actor Object Reference") (OtherComp :type "PrimitiveComponent Object Reference") (OtherBodyIndex :type Integer) (bFromSweep :type Boolean) (SweepResult :type "HitResult Structure (by ref)"))
  (bind _asbp_main_character (cast `/Game/BBB_Vibration_2026/Blueprints/BP_MainCharacter` OtherActor))
  (set `self.As BP Main Character` _asbp_main_character)
  (`SceneComponent.SetVisibility` (`self.Widget`) true false))

(event `self.Sphere.OnComponentEndOverlap`
  (params (OverlappedComponent :type "PrimitiveComponent Object Reference") (OtherActor :type "Actor Object Reference") (OtherComp :type "PrimitiveComponent Object Reference") (OtherBodyIndex :type Integer))
  (cast `/Game/BBB_Vibration_2026/Blueprints/BP_MainCharacter` OtherActor)
  (`/Game/BBB_Vibration_2026/Blueprints/BP_MainCharacter.TakeCollectible` (`self.As BP Main Character`) (`self.Value`) (`self.Adrenaline`) false)
  (`SceneComponent.SetVisibility` (`self.Widget`) false false))

(event `OpenText`
  (`KismetSystemLibrary.PrintString` "Hello")
  (bind _returnvalue (`|CreateWidget` "/Game/BBB_Vibration_2026/Blueprints/Widgets/WBP_Text.WBP_Text_C"))
  (set `/Game/BBB_Vibration_2026/Blueprints/Widgets/WBP_Text.Value` (`self.Index`) _returnvalue)
  (bind _output_get (set `self.NewVar` _returnvalue))
  (`UserWidget.AddToViewport` _output_get 0))

(event `CloseText`
  (`Widget.RemoveFromParent` (`self.NewVar`)))

(fn `UserConstructionScript`
  (bind _plane (`self.Plane`))
  (switch `int` (`self.Index`)
    (:`0`
      (`PrimitiveComponent.SetMaterial` _plane 0 "/Game/BBB_Vibration_2026/Textures/M_Feuille.M_Feuille"))
    (:`1`
      (`PrimitiveComponent.SetMaterial` _plane 0 "/Game/BBB_Vibration_2026/Textures/1_Mat.1_Mat"))
    (:`2`
      (`PrimitiveComponent.SetMaterial` _plane 0 "/Game/BBB_Vibration_2026/Textures/2_Mat.2_Mat"))
    (:`3`
      (`PrimitiveComponent.SetMaterial` _plane 0 "/Game/BBB_Vibration_2026/Textures/3_Mat.3_Mat"))
    (:`4`
      (`PrimitiveComponent.SetMaterial` _plane 0 "/Game/BBB_Vibration_2026/Textures/4_Mat.4_Mat"))
    (:`5`
      (`PrimitiveComponent.SetMaterial` _plane 0 "/Game/BBB_Vibration_2026/Textures/5_Mat.5_Mat"))
    (:`6`
      (`PrimitiveComponent.SetMaterial` _plane 0 "/Game/BBB_Vibration_2026/Textures/6_Mat.6_Mat"))
    (:`7`
      (`PrimitiveComponent.SetMaterial` _plane 0 "/Game/BBB_Vibration_2026/Textures/8_Mat.8_Mat"))
    (:`8`
      (`PrimitiveComponent.SetMaterial` _plane 0 "/Game/BBB_Vibration_2026/Textures/9_Mat.9_Mat"))
    (:`9`
      (`PrimitiveComponent.SetMaterial` _plane 0 "/Game/BBB_Vibration_2026/Textures/10_Mat.10_Mat"))
    (:`10`
      (`PrimitiveComponent.SetMaterial` _plane 0 "/Game/BBB_Vibration_2026/Textures/11_Mat.11_Mat"))
    (:`11`
      (`PrimitiveComponent.SetMaterial` _plane 0 "/Game/BBB_Vibration_2026/Textures/12_Mat.12_Mat"))
    (:`12`
      (`PrimitiveComponent.SetMaterial` _plane 0 "/Game/BBB_Vibration_2026/Textures/13_Mat.13_Mat"))
    (:`13`
      (`PrimitiveComponent.SetMaterial` _plane 0 "/Game/BBB_Vibration_2026/Textures/12_Mat.12_Mat"))
    (:`14`
      (`PrimitiveComponent.SetMaterial` _plane 0 "/Game/BBB_Vibration_2026/Textures/14_Mat.14_Mat"))))