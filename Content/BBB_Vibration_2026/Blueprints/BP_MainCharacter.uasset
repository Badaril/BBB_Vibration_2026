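; BP_MainCharacter is the player character, which emits heartbeat pulses to nearby mobs and drives a weapon component.
; A small overlap sphere, resized to a fixed radius on Tick, tracks BP_Mob actors in TargetInRange.
; While DetectMob is set, a heartbeat-ratio Delay on Tick paces debug-drawn visibility traces, passing the character's mesh location to hit mobs through ReceiveHeartBeat.
; Left and right mouse debug keys call shooting and reloading on BPCWeapon.
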(event OnComponentBeginOverlap(Sphere)
  (params (OverlappedComponent :type Primitive%20Component%20Object%20Reference) (OtherActor :type Actor%20Object%20Reference) (OtherComp :type Primitive%20Component%20Object%20Reference) (OtherBodyIndex :type Integer) (bFromSweep :type Boolean) (SweepResult :type Hit%20Result%20Structure%20%28by%20ref%29))
  (bind _asbp_mob (Utilities|Casting|CastToBP_Mob OtherActor))
  (bind _output_get (Variables|Default|SetAs%20BP%20Mob _asbp_mob))
  (Variables|Default|SetDetectMob true)
  (Development|PrintString "Un mob")
  (Utilities|Array|Add (Variables|Default|GetTargetInRange) _output_get))

(event OnComponentEndOverlap(Sphere)
  (params (OverlappedComponent :type Primitive%20Component%20Object%20Reference) (OtherActor :type Actor%20Object%20Reference) (OtherComp :type Primitive%20Component%20Object%20Reference) (OtherBodyIndex :type Integer))
  (bind _asbp_mob (Utilities|Casting|CastToBP_Mob OtherActor))
  (bind _output_get (Variables|Default|SetAs%20BP%20Mob _asbp_mob))
  (Variables|Default|SetDetectMob false)
  (Utilities|Array|RemoveItem (Variables|Default|GetTargetInRange) _output_get))

(event Input|EnhancedActionEvents|EnhancedInputActionIA_Jump
  (params (ActionValue :type Boolean) (ElapsedSeconds :type Float%20%28double-precision%29) (TriggeredSeconds :type Float%20%28double-precision%29) (InputAction :type Input%20Action%20Object%20Reference :default "/Game/ThirdPerson/Input/Actions/IA_Jump.IA_Jump")))

(event EventBeginPlay
  (Utilities|Array|Clear (Variables|Default|GetTargetInRange)))

(event Collision|EventActorBeginOverlap
  (params (OtherActor :type Actor%20Object%20Reference)))

(event EventTick
  (params (DeltaSeconds :type Float%20%28single-precision%29))
  (Components|Sphere|SetSphereRadius (Variables|Default|GetSphere) 15.0 true)
  (if (Variables|Default|GetDetectMob)
    (Utilities|FlowControl|Delay (/ (Math|Conversions|ToFloat(Integer) (Variables|Default|GetAiming%20Heartbeat)) (Math|Conversions|ToFloat(Integer) (Variables|Default|GetHeartbeat))))
    (for _array_element (Variables|Default|GetTargetInRange)
      (bind _outhit (Collision|LineTraceByChannel (Transformation|GetWorldLocation (Variables|Character|GetMesh)) (Transformation|GetWorldLocation (Variables|/Script/Engine.Actor|GetRootComponent _array_element)) "TraceTypeQuery1" false 0 "ForDuration"))
      (bind _asbp_mob (Utilities|Casting|CastToBP_Mob (.HitActor (Collision|BreakHitResult _outhit))))
      (Default|ReceiveHeartBeat _asbp_mob (Transformation|GetWorldLocation (Variables|Character|GetMesh))))))

(event Input|KeyboardEvents|DebugKeyTab
  (params (Key :type Key%20Structure :default "None") (ActionValue :type Input%20Action%20Value%20Structure)))

(event Input|MouseEvents|DebugKeyLeftMouseButton
  (params (Key :type Key%20Structure :default "None") (ActionValue :type Input%20Action%20Value%20Structure))
  (:Pressed
    (Default|CallShooting (Variables|Default|GetBPC_Weapon))))

(event Input|MouseEvents|DebugKeyRightMouseButton
  (params (Key :type Key%20Structure :default "None") (ActionValue :type Input%20Action%20Value%20Structure))
  (:Pressed
    (Default|CallReloading (Variables|Default|GetBPC_Weapon))))

(fn ConstructionScript
  (|CallParentFunction))

(fn SphereScan)